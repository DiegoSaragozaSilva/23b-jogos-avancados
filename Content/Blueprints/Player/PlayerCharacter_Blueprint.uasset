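; Player Character Blueprint that handles basic player locomotion: jumping, looking and moving.
; The jump input action calls Jump, and the turn and look-up axes feed controller yaw and pitch input.
; Forward and right axes add movement input along vectors built only from control rotation yaw, so movement follows the view horizontally regardless of pitch.
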(event Input|ActionEvents|InputActionPlayer_Jump
  (params (Key :type Key%20Structure :default "None"))
  ;[1 1 1] Jump event
  (:Pressed
    (Character|Jump)))

(event Input|AxisEvents|InputAxisPlayer_Forward
  (params (AxisValue :type Float%20%28single-precision%29))
  ;[1 1 1] Movement Events
  (Pawn|Input|AddMovementInput (Math|Vector|GetForwardVector (Math|Rotator|MakeRotator 0.0 0.0 (.Yaw (Math|Rotator|BreakRotator (Pawn|GetControlRotation :!class /Script/Engine.Pawn))))) AxisValue false))

(event Input|AxisEvents|InputAxisPlayer_Right
  (params (AxisValue :type Float%20%28single-precision%29))
  ;[1 1 1] Movement Events
  (Pawn|Input|AddMovementInput (Math|Vector|GetRightVector (Math|Rotator|MakeRotator 0.0 0.0 (.Yaw (Math|Rotator|BreakRotator (Pawn|GetControlRotation :!class /Script/Engine.Pawn))))) AxisValue false))

(event Input|AxisEvents|InputAxisPlayer_Turn
  (params (AxisValue :type Float%20%28single-precision%29))
  ;[1 1 1] Camera Mouse Events
  (Pawn|Input|AddControllerYawInput AxisValue))

(event Input|AxisEvents|InputAxisPlayer_LookUp
  (params (AxisValue :type Float%20%28single-precision%29))
  ;[1 1 1] Camera Mouse Events
  (Pawn|Input|AddControllerPitchInput AxisValue))

(fn ConstructionScript)