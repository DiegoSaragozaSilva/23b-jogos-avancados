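; Enemy AI Blueprint that roams at random and chases the player when PawnSensing sees a pawn.
; From BeginPlay, RandomRoam moves to reachable points within a fixed radius, retrying immediately on failure or after a random delay on success.
; Seeing any pawn sets IsSeeingPlayer, which is never cleared here, and calls FollowPlayer to AIMoveTo player 0.
; The roam loop has no check on that flag.
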(event OnSeePawn(PawnSensing)
  (params (Pawn :type Pawn%20Object%20Reference))
  (Variables|Default|SetIsSeeingPlayer true)
  (CallFunction|FollowPlayer))

(event Custom|FollowPlayer
  (if (Variables|Default|GetIsSeeingPlayer)
    (AI|AIMoveTo self "0, 0, 0" (Game|GetPlayerCharacter 0) 5.0 false)
    (else
      (CallFunction|RandomRoam))))

(event Custom|Random%20Roam
  (AI|AIMoveTo self (.RandomLocation (AI|Navigation|GetRandomReachablePointinRadius (Transformation|GetActorLocation) 2.5e+03 0 0)) 0 5.0 false
    (:OnSuccess
      (Utilities|FlowControl|Delay (* (Math|Random|RandomFloat) 5.0)))
    (:OnFail
      _))
  (CallFunction|RandomRoam))

(event Collision|EventActorBeginOverlap
  (params (OtherActor :type Actor%20Object%20Reference)))

(event EventBeginPlay
  (CallFunction|RandomRoam))

(fn ConstructionScript)