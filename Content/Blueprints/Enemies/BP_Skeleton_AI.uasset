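; Skeleton enemy AI that roams at random and chases and punches the player on sight.
; Roaming loops AI moves to random reachable nearby points, pausing randomly after each arrival.
; PawnSensing sightings start a chase and refresh a short retriggerable delay that clears the seeing flag.
; Reaching the player plays a punch montage, blocking further chases until it ends, then roaming resumes if sight is lost.
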(event OnSeePawn(PawnSensing)
  (params (Pawn :type Pawn%20Object%20Reference))
  ;[1 1 1] Target follow player and attack
  (Variables|Default|SetIsSeeingPlayer true)
  (Utilities|FlowControl|Sequence
    (:then_0
      (CallFunction|FollowPlayer))
    (:then_1
      (Utilities|FlowControl|RetriggerableDelay 0.6)
      (Variables|Default|SetIsSeeingPlayer false))))

(event Custom|FollowPlayer
  ;[1 1 1] Target follow player and attack
  (if (not (Variables|Default|GetIsAttacking))
    (AI|AIMoveTo self "0, 0, 0" (Game|GetPlayerCharacter 0) 1e+02 false
      (:OnSuccess
        (if (not (Variables|Default|GetIsAttacking))
          (Variables|Default|SetIsAttacking true)
          (bind _returnvalue (Animation|PlayAnimMontage "/Game/Models/Montage_Skeleton_Punching.Montage_Skeleton_Punching" 1.0 "None"))
          (Utilities|FlowControl|Delay _returnvalue)
          (Variables|Default|SetIsAttacking false)
          (if (not (Variables|Default|GetIsSeeingPlayer))
            (CallFunction|RandomRoam))))
      (:OnFail
        (CallFunction|RandomRoam)))))

(event Custom|Random%20Roam
  ;[1 1 1] Random Roaming
  (AI|AIMoveTo self (.RandomLocation (AI|Navigation|GetRandomReachablePointinRadius (Transformation|GetActorLocation) 2.5e+03 0 0)) 0 5.0 false
    (:OnSuccess
      (Utilities|FlowControl|Delay (* (Math|Random|RandomFloat) 5.0)))
    (:OnFail
      _))
  (CallFunction|RandomRoam))

(event Collision|EventActorBeginOverlap
  (params (OtherActor :type Actor%20Object%20Reference)))

(event EventBeginPlay
  ;[1 1 1] Random Roaming
  (CallFunction|RandomRoam))

(fn ConstructionScript)